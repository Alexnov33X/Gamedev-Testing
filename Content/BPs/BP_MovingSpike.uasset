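; BP_MovingSpike is a spike hazard that moves back and forth and kills the player on contact.
; Two alternating timelines, Move and Timeline_0, restart each other endlessly from BeginPlay, stepping the actor along the Cone's up vector, then back.
; Steps are one unit per update without using timeline values, so travel depends on frame rate.
; Cone overlap with the player character calls Death on ThirdPersonCharacter.
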(event OnComponentBeginOverlap(Cone)
  (params (OverlappedComponent :type Primitive%20Component%20Object%20Reference) (OtherActor :type Actor%20Object%20Reference) (OtherComp :type Primitive%20Component%20Object%20Reference) (OtherBodyIndex :type Integer) (bFromSweep :type Boolean) (SweepResult :type Hit%20Result%20Structure%20%28by%20ref%29))
  (bind _returnvalue (Game|GetPlayerCharacter 0))
  ;[1 1 1] Kill player on contact
  (if (== OtherActor _returnvalue)
    (bind _asthird_person_character (Utilities|Casting|CastToThirdPersonCharacter _returnvalue))
    (Default|Death _asthird_person_character)))

(event EventBeginPlay
  (bind _cone (Variables|Default|GetCone))
  (bind _returnvalue (Math|Vector|GetUpVector _cone))
  (Timeline|Move Play
    (:Update
      (Transformation|SetActorLocation (+ (Transformation|GetActorLocation) _returnvalue) false false))
    (:Finished
      (Timeline|Timeline_0 ReverseFromEnd
        (:Update
          (Transformation|SetActorLocation (- (Transformation|GetActorLocation) _returnvalue) false false))
        (:Finished
          (Timeline|Move PlayFromStart))))))

(event Collision|EventActorBeginOverlap
  (params (OtherActor :type Actor%20Object%20Reference)))

(event EventTick
  (params (DeltaSeconds :type Float%20%28single-precision%29)))

(fn ConstructionScript)