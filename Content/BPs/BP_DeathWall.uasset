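; BP_DeathWall is a hazard actor that kills the player on contact and can advance through the level.
; While Moving is set, Tick shifts it along world +X by Speed each frame, without delta-time scaling or sweep.
; An overlap with player pawn 0 casts it to ThirdPersonCharacter and calls its Death function.
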(event EventBeginPlay)

(event Collision|EventActorBeginOverlap
  (params (OtherActor :type Actor%20Object%20Reference))
  (bind _returnvalue (Game|Player|GetPlayerPawn 0))
  (if (== OtherActor _returnvalue)
    (bind _asthird_person_character (Utilities|Casting|CastToThirdPersonCharacter _returnvalue))
    (Default|Death _asthird_person_character)))

(event EventTick
  (params (DeltaSeconds :type Float%20%28single-precision%29))
  (if (Variables|Default|GetMoving)
    (Transformation|SetActorLocation (+ (Transformation|GetActorLocation) (* "1.000000, 0, 0" (Variables|Default|GetSpeed))) false false)))

(fn ConstructionScript)